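; BP_Wind is a short-lived wind actor that carries fire from Fire actors to Combustible actors.
; On overlap it stores the type of any Fire it meets, starting from None, and passes the stored type to any Combustible via SetOnFire.
; Hitting a BP_Obstacles actor destroys it.
; Tick drives a looping half-second Delay that counts SelfDestroyTimer down and destroys the actor when it runs out.
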(event `self.ReceiveBeginPlay`
  (set `self.carriedFireType` "None"))

(event `self.ReceiveActorBeginOverlap`
  (params (OtherActor :type "Actor Object Reference"))
  (bind _asfire (cast `Fire` OtherActor)
    (:`then`
      (set `self.carriedFireType` (`Fire.GetType` _asfire)))
    (:`CastFailed`
      (bind _ascombustible (cast `Combustible` OtherActor)
        (:`then`
          (`Combustible.SetOnFire` _ascombustible (`self.carriedFireType`)))
        (:`CastFailed`
          (cast `/Game/FlowingFire/Blueprints/BP_Obstacles` OtherActor)
          (`self.K2_DestroyActor`))))))

(event `self.ReceiveTick`
  (params (DeltaSeconds :type "Float (single-precision)"))
  ;[1 1 1] Comment
  (`KismetSystemLibrary.Delay` 0.5 :!label _label)
  (if (> (- (`self.SelfDestroyTimer`) 0.5) 0.0)
    (set `self.SelfDestroyTimer` (- (`self.SelfDestroyTimer`) 0.5))
    (goto _label)
    (else
      (`self.K2_DestroyActor`))))

(fn `UserConstructionScript`)