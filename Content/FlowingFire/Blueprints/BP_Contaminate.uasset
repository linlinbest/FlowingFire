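; BP_Contaminate is a contaminated grass actor that becomes purified the first time it finishes burning.
; On that first burn-out, it tints the grass mesh green via a dynamic material, resets its valid fires to red, blue and yellow, and flags itself purified.
; Any later burn-out restarts the current level by reopening it by name.
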(event `self.ReceiveOnBurnOutEnd`
  (if (`self.isPurified`)
    (bind _returnvalue (`GameplayStatics.GetCurrentLevelName` true))
    (`GameplayStatics.OpenLevel` (`KismetStringLibrary.Conv_StringToName` _returnvalue))
    (else
      (bind _returnvalue_2 (`PrimitiveComponent.CreateDynamicMaterialInstance` (`self.Grass_Mesh`) 0 null "None"))
      (`MaterialInstanceDynamic.SetVectorParameterValue` _returnvalue_2 "BaseColor" (struct :`R` 0.206187 :`G` 0.841667 :`B` 0.080036 :`A` 1.0))
      (bind _output_get (set `self.validFire` (`self.validFire`)))
      (`KismetArrayLibrary.Array_Clear` _output_get)
      (`KismetArrayLibrary.Array_Add` _output_get "Red")
      (`KismetArrayLibrary.Array_Add` _output_get "Blue")
      (`KismetArrayLibrary.Array_Add` _output_get "Yellow")
      (set `self.isPurified` true))))

(event `self.ReceiveBeginPlay`)

(fn `UserConstructionScript`)