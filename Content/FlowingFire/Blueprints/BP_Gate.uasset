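; BP_Gate is a level exit gate that opens the FinishLevel map when the FirstPersonCharacter overlaps it while it is passable.
; Until then, Tick checks every entry in TorchFlagArray for a valid current fire.
; Once all are lit, it permanently sets IsPassible, shows its particle system and plays the LevelPass sound.
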(event `self.ReceiveActorBeginOverlap`
  (params (OtherActor :type "Actor Object Reference"))
  (cast `/Game/FirstPersonBP/Blueprints/FirstPersonCharacter` OtherActor)
  (if (`self.IsPassible`)
    (`GameplayStatics.OpenLevel` "FinishLevel")))

(event `self.ReceiveTick`
  (params (DeltaSeconds :type "Float (single-precision)"))
  (if (not (`self.IsPassible`))
    (set `self.ValidNum` 0)
    (for _array_element (`self.torchFlagArray`)
      (`/Engine/EditorBlueprintResources/StandardMacros.IsValid` (`Combustible.GetCurrFire` _array_element)
        (:`Is Valid`
          (set `self.ValidNum` (+ (`self.ValidNum`) 1)))
        (:`Is Not Valid`
          (set `self.IsPassible` false)
          (break))))
    (if (== (`self.ValidNum`) (`KismetArrayLibrary.Array_Length` (`self.torchFlagArray`)))
      (set `self.IsPassible` true)
      (`SceneComponent.SetVisibility` (`self.ParticleSystem`) true false)
      (`GameplayStatics.PlaySound2D` "/Game/Sound/LevelPass.LevelPass" 1.0 1.0 0.0 null null))))

(fn `UserConstructionScript`)