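; Contaminated grass that fire purifies, with each instance counted in FirstPersonGameMode's total on BeginPlay behind a gate used as a lock.
; The first burnout fades the grass green via a timeline, swaps effects, lets pawns overlap, accepts every fire color and increments the purified count.
; Burning purified grass notifies the game mode, and its burnout restarts the current level.
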(event `self.ReceiveBeginPlay`
  ;[1 1 1] update the total number of contaminates in the game
  (`parent.ReceiveBeginPlay`)
  (`/Engine/EditorBlueprintResources/StandardMacros.Gate` false :!label _label
    (:`Exit`
      (`self.BeginModifyContaminatesSum`)
      (bind _asfirst_person_game_mode (cast `/Game/FirstPersonBP/Blueprints/FirstPersonGameMode` (`GameplayStatics.GetGameMode`)))
      (set `/Game/FirstPersonBP/Blueprints/FirstPersonGameMode.contaminatesSum` (+ (`/Game/FirstPersonBP/Blueprints/FirstPersonGameMode.contaminatesSum` _asfirst_person_game_mode) 1) _asfirst_person_game_mode)
      (`self.EndModifyContaminatesSum`))))

(event `EndModifyContaminatesSum`
  ;[1 1 1] update the total number of contaminates in the game
  (goto _label :!via `Open`))

(event `BeginModifyContaminatesSum`
  ;[1 1 1] update the total number of contaminates in the game
  (goto _label :!via `Close`))

(event `PurifyColor`
  ;[1 1 1] Update Color to purified color
  (bind (_direction _colorchangelerptime) (`Timeline|Timeline_ColorChange` :!via `PlayFromStart`)
    (:`Update`
      (bind _returnvalue (`PrimitiveComponent.CreateDynamicMaterialInstance` (`self.Grass_Mesh`) 0 null "None"))
      (bind _returnvalue_2 (`MaterialInstanceDynamic.K2_GetVectorParameterValue` _returnvalue "BaseColor"))
      (`MaterialInstanceDynamic.SetVectorParameterValue` _returnvalue "BaseColor" (`KismetMathLibrary.LinearColorLerp` _returnvalue_2 (struct :`R` 0.206188 :`G` 0.841667 :`B` 0.080036 :`A` 1.0) _colorchangelerptime)))))

(event `self.ReceiveOnBurnOutEnd`
  (if (`self.isPurified`)
    (bind _returnvalue (`GameplayStatics.GetCurrentLevelName` true))
    (`GameplayStatics.OpenLevel` (`KismetStringLibrary.Conv_StringToName` _returnvalue))
    (else
      (`self.PurifyColor`)
      ;[1 1 1] Pawn (player) can overlap with purified contaminates
      (`PrimitiveComponent.SetCollisionResponseToChannel` (`self.Box`) "ECC_Pawn" "ECR_Overlap")
      ;[1 1 1] remove contaminate effect and add purified effect
      (`SceneComponent.SetVisibility` (`self.Contaminated`) false false)
      (`SceneComponent.SetVisibility` (`self.Purified`) true false)
      ;[1 1 1] All fire type become valid on purified contaminates
      (bind _output_get (set `self.validFire` (`self.validFire`)))
      (`KismetArrayLibrary.Array_Clear` _output_get)
      (`KismetArrayLibrary.Array_Add` _output_get "Red")
      (`KismetArrayLibrary.Array_Add` _output_get "Blue")
      (`KismetArrayLibrary.Array_Add` _output_get "Yellow")
      (`KismetArrayLibrary.Array_Add` _output_get "Purple")
      (`KismetArrayLibrary.Array_Add` _output_get "Orange")
      (`KismetArrayLibrary.Array_Add` _output_get "Green")
      (set `self.isPurified` true)
      (bind _asfirst_person_game_mode (cast `/Game/FirstPersonBP/Blueprints/FirstPersonGameMode` (`GameplayStatics.GetGameMode`)))
      (set `/Game/FirstPersonBP/Blueprints/FirstPersonGameMode.purifiedCount` (+ (`/Game/FirstPersonBP/Blueprints/FirstPersonGameMode.purifiedCount` _asfirst_person_game_mode) 1) _asfirst_person_game_mode)
      (`ActorComponent.Activate` (`self.Audio`) false))))

(event `self.ReceiveOnBurnBegin`
  (if (`self.isPurified`)
    (bind _asfirst_person_game_mode (cast `/Game/FirstPersonBP/Blueprints/FirstPersonGameMode` (`GameplayStatics.GetGameMode`)))
    (`/Game/FirstPersonBP/Blueprints/FirstPersonGameMode.OnGrassBurned` _asfirst_person_game_mode)))

(fn `UserConstructionScript`)